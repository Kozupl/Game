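; StoredEquipement_BP holds the data of an equipment item and equips it on a character as a visible part with stat bonuses.
; CopyItemValues copies the gameplay effect spec, rarity, type and look from an item.
; Equip adds a skeletal mesh component attached to the given socket on the character mesh.
; It then applies the spec through the character's Ability System Component and stores the active effect handle.
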(fn Equip
  (params (Character%20 :type Character%20Object%20Reference) (InSocketName :type Name))
  (CallFunction|SetVisiblePart Character%20 InSocketName)
  (CallFunction|ApplyStatsBonusEffect Character%20))

(fn SetVisiblePart
  (params (Equipement%20owner :type Character%20Object%20Reference) (InSocketName :type Name))
  (bind _returnvalue (Game|AddComponentbyClass Equipement%20owner "/Script/Engine.SkeletalMeshComponent" false))
  (Class|SkinnedMeshComponent|SetSkeletalMesh _returnvalue (Variables|Look|GetEquipement%20Look) true)
  (Transformation|AttachComponentToComponent _returnvalue (Variables|/Script/Engine.Character|GetMesh Equipement%20owner) InSocketName "KeepRelative" "KeepRelative" "KeepRelative" true))

(fn ApplyStatsBonusEffect
  (params (Effect%20Target :type Actor%20Object%20Reference))
  (bind _returnvalue (GameplayEffects|ApplyGameplayEffectSpecToSelf (Ability|GetAbilitySystemComponent Effect%20Target) (Variables|Stored|GetEquipement%20Stats)))
  (Variables|Equiped|SetActive%20Effect _returnvalue))

(fn CopyItemValues
  (params (Item :type Equipment%20Component%20BP%20Object%20Reference))
  (Variables|Stored|SetEquipement%20Stats (Variables|/Game/Blueprints/Equipment/EquipmentComponent_BP.EquipmentComponent_BP_C|GetGameplay%20Effect%20Spec Item))
  (Variables|Stored|SetEquipement%20Rarity (Variables|/Game/Blueprints/Equipment/EquipmentComponent_BP.EquipmentComponent_BP_C|GetRarity Item))
  (Variables|Stored|SetEquipenment%20Type (Variables|/Game/Blueprints/Equipment/EquipmentComponent_BP.EquipmentComponent_BP_C|GetItem%20Type Item))
  (Variables|Look|SetEquipement%20Look (Variables|/Game/Blueprints/Equipment/EquipmentComponent_BP.EquipmentComponent_BP_C|GetLook Item)))
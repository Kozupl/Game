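; Loot generator component that spawns randomized equipment drops at its owner's location, then destroys itself.
; Weighted rolls over a drop-chance table choose item types and rarities, creating a loot actor with an equipment component for each success.
; Per-type stat tables, keyed by rarity, feed a capped, cycling roll loop that picks random stat values.
; Stats become SetByCaller magnitudes on a GAS effect spec stored on each forged item.
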(fn GenerateEquipement
  (CallFunction|GenerateLootType)
  (CallFunction|GenerateStats)
  (Components|DestroyComponent))

(fn GenerateLootType
  (bind _out_row (Utilities|ForEachLoopTable (Variables|Default|GetChances%20of%20Loot%20Drop))
    (:then
      (bind _values (Utilities|Map|Values (.DropChance (Utilities|Struct|BreakLootGeneration _out_row))))
      (for (_array_element _array_index) _values
        (if (Math|Random|RandomBoolwithWeight (/ _array_element 1e+02))
          (LocalVariables|SetLoot%20Type (.ItemType (Utilities|Struct|BreakLootGeneration _out_row)))
          (bind _keys (Utilities|Map|Keys (.DropChance (Utilities|Struct|BreakLootGeneration _out_row))))
          (LocalVariables|SetRarity (Utilities|Array|Get(acopy) _keys _array_index))
          (bind _returnvalue (Game|SpawnActorfromClass "/Game/Blueprints/Equipment/Loot_BP.Loot_BP_C" (Math|Transform|MakeTransform (Transformation|GetActorLocation (Components|GetOwner)) "0, 0, 0" "1,1,1") "AdjustIfPossibleButAlwaysSpawn" 0 0))
          (Utilities|Array|Add (Variables|Default|GetGenerated%20equipment) (Actor|GetComponentbyClass _returnvalue "/Game/Blueprints/Equipment/EquipmentComponent_BP.EquipmentComponent_BP_C"))
          (Default|CreateItem (Actor|GetComponentbyClass _returnvalue "/Game/Blueprints/Equipment/EquipmentComponent_BP.EquipmentComponent_BP_C") (LocalVariables|GetLoot%20Type) (LocalVariables|GetRarity)))))))

(fn GenerateStats
  (for _array_element (Variables|Default|GetGenerated%20equipment)
    (bind _returnvalue (Utilities|GetDataTableRow (.Value (Utilities|Map|Find (Variables|Default|GetArmor%20Stats%20Table) (Variables|/Game/Blueprints/Equipment/EquipmentComponent_BP.EquipmentComponent_BP_C|GetItem%20Type _array_element))) (Utilities|String|StringToName (Utilities|String|EnumtoString (Variables|/Game/Blueprints/Equipment/EquipmentComponent_BP.EquipmentComponent_BP_C|GetRarity _array_element))))
      (:then
        (bind _output (CallFunction|GetRandomStats _returnvalue))
        (bind _equip_effect_ (CallFunction|MakeEquipementSpec _output))
        (Variables|/Game/Blueprints/Equipment/EquipmentComponent_BP.EquipmentComponent_BP_C|SetGameplay%20Effect%20Spec _array_element _equip_effect_)
        (Default|EquipementForged _array_element)))))

(fn RandomFloatfromRange
  (params (Float%20Range :type Float%20Range%20Structure))
  (bind (_lowerbound _upperbound) (Utilities|Struct|BreakFloatRange Float%20Range))
  (return (Math|Random|RandomFloatinRange (.Value (Utilities|Struct|BreakFloatRangeBound _lowerbound)) (.Value (Utilities|Struct|BreakFloatRangeBound _upperbound)))))

(fn MakeEquipementSpec
  (params (Stats%20Properties :type Map%20of%20Gameplay%20Tag%20Structures%20to%20Float%20%28single-precision%29s))
  (LocalVariables|SetEquip%20Effect (Utilities|MakeEffectSpec))
  (bind _values (Utilities|Map|Values Stats%20Properties))
  (for (_array_element _array_index) _values
    (bind _keys (Utilities|Map|Keys Stats%20Properties))
    (Ability|GameplayEffect|AssignTagSetbyCallerMagnitude (LocalVariables|GetEquip%20Effect) (Utilities|Array|Get(acopy) _keys _array_index) _array_element))
  (return (LocalVariables|GetEquip%20Effect)))

(fn GetRandomStats
  (params (Stats%20Pattern :type Stats%20Pattern%20Structure))
  (bind (_rarity _statsnumber _stat) (Utilities|Struct|BreakStatsPattern Stats%20Pattern))
  (Utilities|Map|Clear (LocalVariables|GetStat%20Values))
  (Utilities|Map|Values _stat)
  (CallFunction|WhileLoopwithCondition _stat (LocalVariables|GetStat%20Values) _statsnumber 100)
  (return (LocalVariables|GetStat%20Values)))

(fn WhileLoopwithCondition
  (params (TargetMap :type Map%20of%20Gameplay%20Tag%20Structures%20to%20Structs) (Stats :type Map%20of%20Gameplay%20Tag%20Structures%20to%20Float%20%28single-precision%29s) (Last%20Index :type Integer) (Max%20Loop%20Counts :type Integer))
  (bind _values (Utilities|Map|Values TargetMap))
  (LocalVariables|SetLoop%20counts 0)
  (LocalVariables|SetLoop%20Index 0)
  (while (LocalVariables|GetContinue%20Loop)
    (Utilities|FlowControl|Sequence
      (:then_0
        (bind _value_range (Utilities|RollforStat (Utilities|Array|Get(acopy) _values (LocalVariables|GetArray%20Index)))
          (:True
            (bind _returnvalue (CallFunction|RandomFloatfromRange _value_range))
            (bind _keys (Utilities|Map|Keys TargetMap))
            (Utilities|Map|Add Stats (Utilities|Array|Get(acopy) _keys (LocalVariables|GetArray%20Index)) _returnvalue)
            (bind _output_get (LocalVariables|SetLoop%20Index (Utilities|Map|Length Stats)))
            (LocalVariables|SetContinue%20Loop (== _output_get Last%20Index)))))
      (:then_1
        (bind _result (Math|Integer|IncrementInt (LocalVariables|GetArray%20Index))
          (:%20%20
            (if (== _result (- (Utilities|Array|Length _values) 1))
              (LocalVariables|SetArray%20Index 0)
              (bind _result_2 (Math|Integer|IncrementInt (LocalVariables|GetLoop%20counts))
                (:%20%20
                  (LocalVariables|SetContinue%20Loop (not (== _result_2 Max%20Loop%20Counts)))))))))))
  (return))
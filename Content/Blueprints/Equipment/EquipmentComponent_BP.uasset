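; Equipment component that gives its owning actor the look and behavior of a loot item that can be picked up.
; When forged, it adds a skeletal mesh with a random pick from PossibleLooks, set to block, plus a LootName component above it.
; PickUp passes the owner to the interacting actor's Inventory_BP component.
; CreateItem stores type and rarity; SetCollision adds a sphere but is uncalled here and partly unwired.
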(event Custom|Equipement%20Forged
  ;[0 0 0] Begin Play
  (CallFunction|SetLook)
  (CallFunction|AddText))

(event Custom|Pick%20Up
  (params (Interacting%20actor :type Actor%20Object%20Reference))
  (bind _returnvalue (Actor|GetComponentbyClass Interacting%20actor "/Game/Blueprints/Equipment/Inventory_BP.Inventory_BP_C"))
  ;[0 0 0] Equip
  (Utilities|IsValid _returnvalue
    (:Is%20Valid
      (Default|PickUp _returnvalue (Components|GetOwner)))))

(fn SetCollision
  (bind _returnvalue (Components|GetOwner))
  (Game|AddComponentbyClass _returnvalue "/Script/Engine.SphereComponent" false (Math|Conversions|ToTransform(Vector) (Transformation|GetActorLocation _returnvalue))))

(fn CreateItem
  (params (Item%20Type :type Gameplay%20Tag%20Structure) (Rarity :type LootRarity%20Enum :default "NewEnumerator0"))
  (Variables|Attributes|SetItem%20Type Item%20Type)
  (Variables|Attributes|SetRarity Rarity))

(fn SetLook
  (bind _result (Utilities|Set|ToArray (Variables|Components|GetPossible%20looks)))
  (bind _returnvalue (Game|AddComponentbyClass (Components|GetOwner) "/Script/Engine.SkeletalMeshComponent" false))
  (bind _output_get (Variables|Look|SetLook (Utilities|Array|Get(acopy) _result (Math|Random|RandomIntegerinRange 0 (Utilities|Array|LastIndex _result)))))
  (Class|SkinnedMeshComponent|SetSkeletalMesh _returnvalue _output_get false)
  (Collision|SetCollisionObjectType _returnvalue "ECC_GameTraceChannel1")
  (Collision|SetCollisionEnabled _returnvalue "QueryAndPhysics")
  (Collision|SetCollisionResponsetoAllChannels _returnvalue "ECR_Block"))

(fn AddText
  (bind _returnvalue (Game|AddComponentbyClass (Components|GetOwner) "/Game/Blueprints/Equipment/Widgets/LootName.LootName_C" false (Math|Transform|MakeTransform "0.000000, 0,200.000000" "0,180.000000, 0")))
  (bind _output_get (Variables|Default|SetLoot%20Name _returnvalue))
  (Collision|SetCollisionObjectType _output_get (Variables|Components|Collision|GetCollision%20Channel)))
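; Inventory component that handles item pickup and automatic equipping on the owning character.
; Picked-up actors become StoredEquipement_BP objects in the inventory and are destroyed.
; A breakable macro tag-matches equipment type to slots, stopping at an empty one, then Equip swaps out any occupant and passes the slot's socket to the item.
; Removal clears the piece's Gameplay Ability System effect and returns it to the inventory.
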(event Custom|Pick%20Up
  (params (Item :type Actor%20Object%20Reference%20%28by%20ref%29))
  ;[0 0 0] Pick up
  (bind _stored_equipement (CallFunction|StoreItem Item))
  (bind _item_index (Utilities|AddItemtoInventory _stored_equipement))
  (bind _matching_tag (Utilities|FindItem'sSlot _stored_equipement :!label _label)
    (:Completed
      (CallFunction|Equip _stored_equipement _matching_tag _item_index))
    (:Has%20matches%20tag
      (Utilities|IsValid (.Value (Utilities|Map|Find (Variables|Default|GetEquiped%20items) _matching_tag))
        (:Is%20Not%20Valid
          (goto _label Break))))))

(fn RemoveEquipement
  (params (Equipement%20Piece :type Stored%20Equipement%20BP%20Object%20Reference%20%28by%20ref%29) (Slot :type Gameplay%20Tag%20Structure%20%28by%20ref%29))
  (Utilities|FlowControl|Sequence
    (:then_0
      (GameplayEffects|RemoveActiveGameplayEffect (Utilities|GetOwner'sAbilitySystemComponent) (Variables|/Game/Blueprints/Equipment/StoredEquipement_BP.StoredEquipement_BP_C|GetActive%20Effect Equipement%20Piece) -1)
      (Utilities|Array|Add (Variables|Default|GetInventory) Equipement%20Piece) ; Hope They Added To End
    )
    (:then_1
      (Utilities|Map|Add (Variables|Default|GetEquiped%20items) Slot 0))))

(fn WearEquipementPiece
  (params (New%20Equipement :type Actor%20Object%20Reference))
  (GameplayEffects|ApplyGameplayEffectSpecToSelf (Utilities|GetOwner'sAbilitySystemComponent) (Variables|/Game/Blueprints/Equipment/EquipmentComponent_BP.EquipmentComponent_BP_C|GetGameplay%20Effect%20Spec (Actor|GetComponentbyClass New%20Equipement "/Game/Blueprints/Equipment/EquipmentComponent_BP.EquipmentComponent_BP_C"))))

(fn StoreItem
  (params (Item :type Actor%20Object%20Reference))
  (bind _returnvalue (Game|ConstructObjectfromClass "/Game/Blueprints/Equipment/StoredEquipement_BP.StoredEquipement_BP_C" self))
  (Default|CopyItemValues _returnvalue (Actor|GetComponentbyClass Item "/Game/Blueprints/Equipment/EquipmentComponent_BP.EquipmentComponent_BP_C"))
  (Actor|DestroyActor Item)
  (return _returnvalue))

(fn Equip
  (params (Item :type Stored%20Equipement%20BP%20Object%20Reference) (Slot :type Gameplay%20Tag%20Structure :default "(TagName=\"Equipment\")") (Index :type Integer))
  (bind (_value _item_found) (Utilities|GetEquipedIteminSlot Slot))
  (Utilities|FlowControl|Sequence
    (:then_0
      (if _item_found
        (CallFunction|RemoveEquipement _value Slot)))
    (:then_1
      (Default|Equip Item (.AsCharacter (Utilities|Casting|CastToCharacter (Components|GetOwner))) (.Value (Utilities|Map|Find (Variables|Default|GetEquipement%20Sockets) Slot)))
      (Utilities|Array|RemoveIndex (Variables|Default|GetInventory) Index)
      (Utilities|Map|Add (Variables|Default|GetEquiped%20items) Slot Item))))
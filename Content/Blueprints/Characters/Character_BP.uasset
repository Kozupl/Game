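; Character Blueprint built on the Gameplay Ability System, with spell, dash and auto-attack abilities, a health bar and a bounty applied to the killer on death.
; BeginPlay starts an async attribute listener, grants the default abilities with array index as input code, and applies health and mana regen effects.
; Spell and dash activate by class, while auto-attack sends a gameplay event carrying the target.
; Health and move-speed handlers update the widget and walk speed.
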(event Custom|Health%20Changed
  (params (New%20value :type Float%20%28single-precision%29) (NewParam :type Gameplay%20Attribute%20Structure))
  ;[0 1 0.03529] Current Health change
  (Utilities|UpdateHealthBar New%20value))

(event Custom|Move%20Speed%20Changed
  (params (New%20Value :type Float%20%28single-precision%29))
  ;[0 1 0.03529] Move Speed Changed
  (Variables|/Script/Engine.CharacterMovementComponent|SetMaxWalkSpeed (Variables|Character|GetCharacterMovement) New%20Value))

(event EventAttackTarget
  (params (ASC :type Ability%20System%20Component%20Object%20Reference))
  ;[1 0.1406 0.1406] AutoAttack (note: get rid of this)
  (CallFunction|ActivateAbilityThroughtEvent "(TagName=\"Triggers.Attack\")" (Components|GetOwner ASC) 0.0))

(event EventUseAbility
  ;[0 0 0] Cast Ability
  (Abilities|TryActivateAbilitybyClass (Variables|Default|GetAbilitySystemComponent) (Variables|Abilities|GetSpellAbility) true))

(event EventDie
  (params (Killer :type Actor%20Object%20Reference))
  ;[0 0 0] Die
  (GameplayEffects|ApplyGameplayEffectToTarget :self (Variables|Default|GetAbilitySystemComponent) :GameplayEffectClass "/Game/Blueprints/Gameplay_Effects/Bounty_Effect.Bounty_Effect_C" :Target (Ability|GetAbilitySystemComponent Killer)) ; Bounty Effect Apply
  (|CallParentFunction Killer))

(event EventDestroyed
  ;[0.2648 0.4932 0.9844] OnDeath
  (CallFunction|EndTaskifValid (Variables|Attributes|Listening|GetListen%20for%20attribute%20change%20task)))

(event EventBeginPlay
  ;[0 0 0] Begin Play
  (bind (_asynctaskproxy _attribute _newvalue _oldvalue) (|ListenforAttributesChange (Variables|Default|GetAbilitySystemComponent) (Variables|Default|GetAttributesToListen))
    (:then
      (Variables|Attributes|Listening|SetListen%20for%20attribute%20change%20task _asynctaskproxy)
      (CallFunction|SetDefaultAbilities)
      (GameplayEffects|ApplyGameplayEffectToSelf :self (Variables|Default|GetAbilitySystemComponent) :GameplayEffectClass "/Game/Blueprints/Gameplay_Effects/HealthRegen_Effect.HealthRegen_Effect_C")
      (GameplayEffects|ApplyGameplayEffectToSelf :self (Variables|Default|GetAbilitySystemComponent) :GameplayEffectClass "/Game/Blueprints/Gameplay_Effects/ManaRegen_Effect.ManaRegen_Effect_C"))
    (:OnAttributeChanged
      (Default|CallAttributeChanged _attribute _newvalue _oldvalue))))

(event EventUseDash
  ;[0 0 0] Use Dash
  (Abilities|TryActivateAbilitybyClass (Variables|Default|GetAbilitySystemComponent) (Variables|Abilities|GetDashAbility) true))

(fn ConstructionScript)

(fn SetTarget
  (params (InputPin :type Ability%20System%20Component%20Object%20Reference))
  (if (!= (Variables|Default|GetAbilitySystemComponent) InputPin)
    (if (not (!= (Components|GetOwner InputPin) 0))
      (return false))
    (else
      (return false))))

(fn SetDefaultAbilities
  (for (_array_element _array_index) (Variables|Default|GetCharacterAbilities)
    (Class|GameCharacter|GrandAbility _array_element 1 _array_index)))

(fn ActivateAbilityThroughtEvent
  (params (Event%20Tag :type Gameplay%20Tag%20Structure) (Target :type Actor%20Object%20Reference) (Event%20Magnitude :type Float%20%28single-precision%29))
  (Ability|SendGameplayEventtoActor self "(TagName=\"Triggers.Attack\")" (Utilities|MakeTargetDataPayload Event%20Tag Target Event%20Magnitude)))

(fn GetCastPoint
  (return (Variables|Default|GetSpell%20Cast%20Point)))

(fn EndTaskifValid
  (params (InputPin :type Async%20Task%20Attribute%20Changed%20Object%20Reference))
  (Utilities|IsValid InputPin
    (:Is%20Valid
      (Class|AsyncTaskAttributeChanged|EndTask InputPin))))

(fn Test)
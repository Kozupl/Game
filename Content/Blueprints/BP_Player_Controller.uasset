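; Player controller for click-to-move play with Gameplay Ability System integration, forwarding cast and dash input to the pawn.
; SetDestination input tries the pickup ability; a cancellation event classifies the actor under the cursor as ability-system, interactive or other, then moves to the hit location.
; RotatePawn stops movement and opens a Tick gate that interpolates yaw toward the target, then sends Rotation.Over and closes.
; Helpers cover range checks, including attribute-based attack range.
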(event Custom|Begin%20Move
  (params (Target%20Location :type Vector))
  ;[0 0 0] Begin Move
  (Movement|MovePawntoLocation Target%20Location))

(event EventAbilityWasCanceled
  (params (Was%20Canceled :type Boolean))
  (bind _hitresult (Game|Player|GetHitResultUnderCursorbyChannel "TraceTypeQuery2" false))
  (bind (_bblockinghit _binitialoverlap _time _distance _location _impactpoint _normal _impactnormal _physmat _hitactor) (Collision|BreakHitResult _hitresult))
  ;[0 0 0] Set Destination (Right Mouse Button)
  (if Was%20Canceled
    (Movement|SetDestination _hitactor _location)))

(event EventRotatePawn
  (params (Target%20Location :type Vector :default "0, 0, 0"))
  ;[0.2817 0.02875 0.5521] Rotate Pawn
  (Actions|CancelActions)
  (Variables|Dump|SetMovement%20State "NewEnumerator3")
  (Utilities|SetTargetRotation Target%20Location)
  ;[0 0 0] Comment
  (Utilities|FlowControl|Gate true) ; enters at Open
)

(event EventTick
  (params (DeltaSeconds :type Float%20%28single-precision%29))
  ;[0 0 0] Comment
  (Utilities|FlowControl|Gate true :!label _label
    (:Exit
      (Transformation|SetActorRotation (Pawn|GetControlledPawn) (Utilities|InterpolateRotation DeltaSeconds (Variables|Rotation|GetTarget%20Rotation)))
      (if (Utilities|IsPawnRotating (Variables|Rotation|GetTarget%20Rotation) 0.01)
        (Ability|SendGameplayEventtoActor (Pawn|GetControlledPawn) "(TagName=\"Triggers.Rotation.Over\")")
        (goto _label Close)))))

(event EventStopAllActions
  ;[0.5899 0.06042 1] Cancel All Actions
  (Actions|CancelActions)
  ;[0 0 0] Comment
  (Utilities|FlowControl|Gate true) ; enters at Close
)

(event Input|ActionEvents|InputActionStop
  (params (Key :type Key%20Structure))
  ;[0 0 0] Cancel (S button)
  (:Pressed
    (CallFunction|StopAllActions)))

(event Input|ActionEvents|InputActionCastAbility
  (params (Key :type Key%20Structure))
  ;[0 0 0] Cast Spell (mb add direction check here, instead of in the ability)
  (:Pressed
    (Class|CharactersInterface|UseAbility(Message) (Pawn|GetControlledPawn))))

(event Input|ActionEvents|InputActionSetDestination
  (params (Key :type Key%20Structure))
  ;[0 0 0] Set Destination (Right Mouse Button)
  (:Pressed
    (Abilities|TryActivateAbilitybyClass (Ability|GetAbilitySystemComponent (Pawn|GetControlledPawn)) "/Game/Blueprints/Abilities/PickUpItem_GA.PickUpItem_GA_C" true)))

(event Input|ActionEvents|InputActionDash
  (params (Key :type Key%20Structure))
  ;[0 0 0] Use Dash (Space button)
  (:Pressed
    (Class|CharactersInterface|UseDash(Message) (Pawn|GetControlledPawn))))

(fn ConstructionScript)

(fn MovePawntoLocation
  (params (Goal :type Vector%20%28by%20ref%29))
  (AI|Navigation|SimpleMovetoLocation self Goal))

(fn MovePawntoActor
  (AI|Navigation|SimpleMovetoActor self (Variables|Actions|GetTarget%20Actor)))

(fn CancelActions
  (Variables|Actions|SetTarget%20Actor 0)
  (Variables|Rotation|SetTarget%20Rotation "0, 0, 0")
  (AI|Navigation|StopMovement))

(fn IsinRange
  (params (Target%20Location :type Vector))
  (return (> (Variables|Actions|GetPickup%20Range) (Math|Vector|VectorLength (- Target%20Location (Transformation|GetActorLocation))))))

(fn SetDestination
  (params (Hit%20Actor :type Actor%20Object%20Reference) (Location :type Vector))
  (Utilities|IsValid Hit%20Actor
    (:Is%20Valid
      (Utilities|FlowControl|Sequence
        (:then_0
          (Utilities|IsValid (Ability|GetAbilitySystemComponent Hit%20Actor)
            (:Is%20Valid
              (Variables|Dump|SetMovement%20State "NewEnumerator1")
              (Variables|Actions|SetTarget%20Actor Hit%20Actor))
            (:Is%20Not%20Valid
              (if (Utilities|DoesObjectImplementInterface Hit%20Actor "/Game/Blueprints/Interfaces/Interactive_Interface_BP.Interactive_Interface_BP_C")
                (Variables|Dump|SetMovement%20State "NewEnumerator4")
                (Variables|Actions|SetTarget%20Actor Hit%20Actor)
                (else
                  (Variables|Dump|SetMovement%20State "NewEnumerator0")
                  (Variables|Actions|SetTarget%20Actor 0))))))
        (:then_1
          (CallFunction|BeginMove Location))))))
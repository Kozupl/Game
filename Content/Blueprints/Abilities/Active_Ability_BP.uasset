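; Base Gameplay Ability for active abilities, with shared helpers for rotating, approaching a target, cooldowns and montage playback.
; Rotation messages the pawn and waits for a gameplay event before calling RotationIsOver, with that task ended on ability end.
; Approach uses SimpleMoveToActor and a runtime CastRange sphere whose overlap is meant to stop movement and call TargetInRange.
; Activation and both callbacks are empty hooks; cooldown comes from a float or attribute.
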(event Custom|Call%20Pawn%20To%20Rotate
  (params (Target%20Pawn :type Controller%20Object%20Reference) (Rotate%20To%20 :type Vector))
  ;[0 0 0] Rotate Pawn
  (Class|ControllerInterfaceBP|RotatePawn(Message) Target%20Pawn Rotate%20To%20)
  (bind _asynctaskproxy (Ability|Tasks|WaitGameplayEvent "(TagName=\"Triggers.Rotation.Over\")" 0)
    (:then
      (Variables|Cleanup|SetRotation%20Trigger _asynctaskproxy))
    (:EventReceived
      (CallFunction|RotationIsOver Rotate%20To%20))))

(event Custom|Cleanup
  ;[0.2392 0 0.3373] Cleanup
  (CallFunction|EndTaskifValid (Variables|Cleanup|GetRotation%20Trigger)))

(event Custom|Rotation%20Is%20Over
  (params (Target%20Location :type Vector)))

(event Custom|Move%20to%20target
  (params (Target :type Actor%20Object%20Reference%20%28by%20ref%29))
  ;[0 0 0] Move Until In Range (mb change this when after I made CharacterMovingComp)
  (Variables|TargetChasing|SetTarget Target)
  (AI|Navigation|SimpleMovetoActor (Utilities|GetController) (Variables|TargetChasing|GetTarget))
  (bind _returnvalue (CallFunction|CreateCollisionSphere))
  (Collision|AssignOnComponentBeginOverlap _returnvalue (delegate Custom|On%20Possible%20Target%20In%20Range)))

(event Custom|On%20Possible%20Target%20In%20Range
  (params (OverlappedComponent :type Primitive%20Component%20Object%20Reference) (OtherActor :type Actor%20Object%20Reference) (OtherComp :type Primitive%20Component%20Object%20Reference) (OtherBodyIndex :type Integer) (bFromSweep :type Boolean) (SweepResult :type Hit%20Result%20Structure%20%28by%20ref%29))
  ;[0 0 0] Move Until In Range (mb change this when after I made CharacterMovingComp)
  (if (== (Variables|TargetChasing|GetTarget) OverlappedComponent)
    (AI|Navigation|StopMovement (Utilities|GetController))
    (CallFunction|TargetinRange)))

(event Custom|Target%20In%20Range)

(event Ability|EventActivateAbility
  ;[0 0 0] Activate Ability
)

(event Ability|EventOnEndAbility
  (params (bWasCancelled :type Boolean))
  ;[0 0 0] End Ability
  (CallFunction|Cleanup))

(fn SetCooldown
  (params (Based%20On%20Attribute :type Magnitude_Value%20Enum :default "NewEnumerator0") (New%20Value :type Float%20%28single-precision%29) (Attribute :type Gameplay%20Attribute%20Structure))
  (bind _returnvalue (Ability|GetAbilitySystemComponentfromActorInfo))
  (bind _cooldownduration (Variables|Default|GetCooldownDuration))
  (bind (_value _curve _registrytype) (Utilities|Struct|BreakScalableFloat _cooldownduration))
  (bind (_bsuccessfullyfoundattribute _returnvalue_2) (Ability|Attribute|GetFloatAttributefromAbilitySystemComponent _returnvalue Attribute))
  (switch Utilities|FlowControl|Switch|SwitchonMagnitude_Value Based%20On%20Attribute
    (:NewEnumerator0
      (if _bsuccessfullyfoundattribute
        (Class|ActiveAbility|SetCooldownDuration (Utilities|Struct|MakeScalableFloat _returnvalue_2 _curve _registrytype))
        (else
          (Development|PrintString "Attribute not found"))))
    (:NewEnumerator1
      (Class|ActiveAbility|SetCooldownDuration (Utilities|Struct|MakeScalableFloat New%20Value _curve _registrytype)))))

(fn EndTaskifValid
  (params (Asynk%20Task :type Gameplay%20Task%20Object%20Reference))
  (Utilities|IsValid Asynk%20Task
    (:Is%20Valid
      (GameplayTasks|EndTask Asynk%20Task))))

(fn IsinRange
  (params (Target :type Actor%20Object%20Reference))
  (return (>= (Variables|Attributes|GetCast%20Range%20) (Math|Vector|Distance2D(Vector) (Transformation|GetActorLocation Target) (Transformation|GetActorLocation (Ability|GetAvatarActorfromActorInfo))))))

(fn CreateCollisionSphere
  (bind _returnvalue (Game|AddComponentbyClass (Ability|GetAvatarActorfromActorInfo) "/Script/Engine.SphereComponent" false))
  (Components|Sphere|SetSphereRadius _returnvalue (Variables|Attributes|GetCast%20Range%20) true)
  (Collision|SetCollisionResponsetoAllChannels _returnvalue "ECR_Ignore")
  (Collision|SetCollisionResponsetoChannel _returnvalue (Variables|TargetChasing|GetCollision%20Chanel) (Variables|TargetChasing|GetResponse))
  (Rendering|SetVisibility _returnvalue true false)
  (return _returnvalue))
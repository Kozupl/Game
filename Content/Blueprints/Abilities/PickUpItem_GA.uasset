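; Gameplay ability for picking up items, currently a stub: its activate, end and target-in-range events are all empty.
; Disconnected nodes sketch the flow: trace under the cursor, check the hit actor for a component, then pick it up if in range or move to it.
; That unwired logic cancels on an invalid hit, with separate fragments for a direct pickup and for reporting cancellation to the player controller.
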(event Ability|EventActivateAbility
  ;[0 0 0] Activate Ability
)

(event EventTargetinRange)

(event Ability|EventOnEndAbility
  (params (bWasCancelled :type Boolean))
  ;[0 0 0] On End Ability
)
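; Gameplay Ability for an attack that applies a Gameplay Effect to the event's target.
; Activation sets an attribute-based cooldown, commits, then waits for a Triggers.Attack event.
; The event plays a random left or right montage section, slowed for longer cooldowns, and its notify applies the effect and ends the ability.
; Cleanup ends the wait task; a range-check graph is defined but not called here.
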(event Ability|EventActivateAbility
  ;[0 0 0] Activate Ability
  (CallFunction|SetCooldown "NewEnumerator0" 0.0 "(AttributeName=\"AttackSpeed\",Attribute=/Script/Game.GameAttributeSet:AttackSpeed,AttributeOwner=None)")
  (Ability|CommitAbility)
  (bind (_asynctaskproxy _payload) (Ability|Tasks|WaitGameplayEvent "(TagName=\"Triggers.Attack\")" 0 true false)
    (:then
      (Variables|Cleanup|SetAsync%20Task _asynctaskproxy))
    (:EventReceived
      (Utilities|PlayAnimation
        (:On%20Notify%20Begin
          (GameplayEffects|ApplyGameplayEffectToTarget (.TargetData (Utilities|Struct|BreakGameplayEventData _payload)) (Variables|Default|GetGameplay%20Effect%20Class) 1 1)
          (Ability|EndAbility))))))

(event EventCleanup
  (|CallParentFunction)
  (CallFunction|EndTaskifValid (Variables|Cleanup|GetAsync%20Task)))
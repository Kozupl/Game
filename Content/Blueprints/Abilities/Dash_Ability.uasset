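; Gameplay Ability that dashes the avatar toward the point under the player's cursor.
; Activation commits, clamps the cursor hit to CastRange in 2D, shortens it at any Visibility trace hit, and requests pawn rotation.
; RotationIsOver then plays a montage rate-scaled to EffectDuration and starts an ApplyRootMotionMoveToForce task to the target.
; The ability ends when that task times out, and Cleanup ends any remaining task.
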(event Ability|EventActivateAbility
  ;[0 0 0] Activate Ability
  (Ability|CommitAbility)
  (CallFunction|GroundTarget))

(event EventRotationIsOver
  (params (Target%20Location :type Vector :default "0, 0, 0"))
  ;[0 0 0] Rotation Is Over
  (Utilities|PlayAnimation)
  (bind _asynctaskproxy (Ability|Tasks|ApplyRootMotionMoveToForce "None" Target%20Location (Variables|Default|GetEffect%20Duration) false "MOVE_None" false 0 "MaintainLastRootMotionVelocity")
    (:then
      (Variables|Default|SetRoot%20Motion%20Task _asynctaskproxy))
    (:OnTimedOut
      (Ability|EndAbility :!label _label))
    (:OnTimedOutAndDestinationReached
      (goto _label))))

(event EventCleanup
  ;[0.2392 0 0.3373] Cleanup
  (|CallParentFunction)
  (CallFunction|EndTaskifValid (Variables|Default|GetRoot%20Motion%20Task)))

(fn GroundTarget
  (bind _returnvalue (Ability|GetActorInfo))
  (bind _hitresult (Game|Player|GetHitResultUnderCursorbyChannel (.playercontroller _returnvalue) "TraceTypeQuery2" false))
  (bind (_bblockinghit _binitialoverlap _time _distance _location) (Collision|BreakHitResult _hitresult))
  (if _bblockinghit
    (bind _return (CallFunction|CalculateLocation _location))
    (bind (_outhit _returnvalue_2) (Collision|LineTraceByChannel (Transformation|GetActorLocation (Ability|GetAvatarActorfromActorInfo)) _return "TraceTypeQuery1" false 0 "None"))
    (if _returnvalue_2
      (CallFunction|CallPawntoRotate (.playercontroller _returnvalue) (.Location (Collision|BreakHitResult _outhit)))
      (return (.Location (Collision|BreakHitResult _outhit)))
      (else
        (CallFunction|CallPawntoRotate (.playercontroller _returnvalue) (.TraceEnd (Collision|BreakHitResult _outhit)))
        (return (.TraceEnd (Collision|BreakHitResult _outhit)))))))

(fn CalculateLocation
  (params (Target%20location :type Vector))
  (bind (_x _y _z) (Math|Vector|BreakVector Target%20location))
  (bind _returnvalue (Ability|GetAvatarActorfromActorInfo))
  (bind _cast_range_ (Variables|Default|GetCast%20Range%20))
  (bind (_x_2 _y_2) (Math|Vector|BreakVector Target%20location))
  (bind _returnvalue_2 (Transformation|GetActorLocation _returnvalue))
  (bind _returnvalue_3 (Math|Vector|Distance2D(Vector) (Math|Vector2D|MakeVector2D _x _y) (Math|Vector2D|MakeVector2D (.x _returnvalue_2) (.y _returnvalue_2))))
  (if (> _returnvalue_3 _cast_range_)
    (bind (_y_3 _x_3) (CallFunction|FindPointonVectorWhithLenght _returnvalue_3 _cast_range_ (Math|Vector2D|MakeVector2D (.x _returnvalue_2) (.y _returnvalue_2)) (Math|Vector2D|MakeVector2D _x_2 _y_2)))
    (return (Math|Vector|MakeVector _x_3 _y_3 _z))
    (else
      (return Target%20location))))

(fn FindPointonVectorWhithLenght
  (params (Current%20Lenght :type Float%20%28single-precision%29) (Wanted%20Length :type Float%20%28single-precision%29) (Vector%20Start%20Point :type Vector%202D%20Structure) (Vector%20End%20Point :type Vector%202D%20Structure))
  (bind _returnvalue (CallFunction|FindNewPoint Current%20Lenght Wanted%20Length (Math|Vector2D|MakeVector2D (.x Vector%20Start%20Point) (.x Vector%20End%20Point))))
  (bind _returnvalue_2 (CallFunction|FindNewPoint Current%20Lenght Wanted%20Length (Math|Vector2D|MakeVector2D (.y Vector%20Start%20Point) (.y Vector%20End%20Point))))
  (return _returnvalue_2 _returnvalue))

(fn FindNewPoint
  (params (Current%20Lenght :type Float%20%28single-precision%29) (Wanted%20Lenght :type Float%20%28single-precision%29) (Vector%20Start/End%20Point :type Vector%202D%20Structure))
  (bind (_x _y) (Math|Vector2D|BreakVector2D Vector%20Start/End%20Point))
  (bind _output_get (LocalVariables|Setsin%28alfa%29 (/ (Math|Float|Absolute(Float) (- _x _y)) Current%20Lenght)))
  (if (> _x _y)
    (return (- _x (* _output_get Wanted%20Lenght)))
    (else
      (return (+ (* _output_get Wanted%20Lenght) _x)))))